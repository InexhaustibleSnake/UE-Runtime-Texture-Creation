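; First-person style player character that previews and places textured decals on surfaces in the level.
; Each tick, a visibility trace from the player viewpoint moves the runtime preview decal to the hit point, oriented along its normal.
; Setters update the preview's texture through a dynamic material and its clamped size.
; Input handles movement, look, toggling the preview and spawning decals, each with its own dynamic material instance.
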(event `self.ReceiveTick`
  (params (DeltaSeconds :type "Float (single-precision)"))
  (bind (_returnvalue_bblockinghit _returnvalue_binitialoverlap _returnvalue_time _returnvalue_distance _returnvalue_location _returnvalue_impactpoint _returnvalue_normal) (`GameplayStatics.BreakHitResult` (`self.GetForwardTraceData`)))
  ; Event Tick
  (bind _isrtruntimedecalcomponent (`self.ISRTRuntimeDecalComponent`)
    (:`then`
      (`SceneComponent.K2_SetWorldLocationAndRotation` _isrtruntimedecalcomponent _returnvalue_impactpoint (`KismetMathLibrary.Conv_VectorToRotator` _returnvalue_normal) false false))
    (:`else`)))

(event `self.ReceiveBeginPlay`
  ; Begin Play
  (bind _returnvalue (`KismetMaterialLibrary.CreateDynamicMaterialInstance` "/Game/IsRuntimeTexture/Player/MI_PlayerDecal.MI_PlayerDecal"))
  (set `self.PlayerDecalMaterial` _returnvalue)
  (bind _isrtruntimedecalcomponent (`self.ISRTRuntimeDecalComponent`)
    (:`then`
      (`DecalComponent.SetDecalMaterial` _isrtruntimedecalcomponent (`self.PlayerDecalMaterial`))
      (`self.SetDecalSize` (`self.DecalSize`)))
    (:`else`)))

(event `InputAxis|MoveForward`
  (params (AxisValue :type "Float (single-precision)"))
  ; Movement
  (`self.AddMovementInput` (`self.GetActorForwardVector`) AxisValue))

(event `InputAxis|MoveRight`
  (params (AxisValue :type "Float (single-precision)"))
  ; Movement
  (`self.AddMovementInput` (`self.GetActorRightVector`) AxisValue))

(event `InputAxis|MouseX`
  (params (AxisValue :type "Float (single-precision)"))
  ; Mouse
  (`self.AddControllerYawInput` AxisValue))

(event `InputAxis|MouseY`
  (params (AxisValue :type "Float (single-precision)"))
  ; Mouse
  (`self.AddControllerPitchInput` AxisValue))

(event `InputAction|SpawnDecal`
  (params (Key :type "Key Structure"))
  ; Decal Creation
  (:`Pressed`
    (`self.CreateDecal`)))

(event `InputAction|HidePlayerDecal`
  (params (Key :type "Key Structure"))
  ; Hide Decal
  (:`Pressed`
    (bind _isrtruntimedecalcomponent (`self.ISRTRuntimeDecalComponent`)
      (:`then`
        (`SceneComponent.SetVisibility` _isrtruntimedecalcomponent (not (`SceneComponent.IsVisible` (`self.ISRTRuntimeDecalComponent`))) false))
      (:`else`))))

(fn `CreateDecal`
  (locals (DecalMaterial :type "MaterialInstanceDynamic Object Reference"))
  (bind (_bblockinghit _binitialoverlap _time _distance _location _impactpoint _normal) (`GameplayStatics.BreakHitResult` (`self.GetForwardTraceData`)))
  (bind _returnvalue (`KismetMaterialLibrary.CreateDynamicMaterialInstance` "/Game/IsRuntimeTexture/Player/MI_LevelRuntimeDecal.MI_LevelRuntimeDecal"))
  (bind _output_get (set `local.DecalMaterial` _returnvalue))
  (`/Engine/EditorBlueprintResources/StandardMacros.IsValid` _output_get
    (:`Is Valid`
      (`MaterialInstanceDynamic.SetTextureParameterValue` (`local.DecalMaterial`) "Texture" (`self.SelectedTexture`))
      (`GameplayStatics.SpawnDecalAtLocation` (`local.DecalMaterial`) (`KismetMathLibrary.Conv_DoubleToVector` (`self.GetDecalSize`)) _impactpoint (`KismetMathLibrary.Conv_VectorToRotator` _normal)))))

(fn `GetDecalSize`
  (returns (ReturnValue :type "Float (double-precision)"))
  (return (`self.DecalSize`)))

(fn `GetForwardTraceData`
  (returns (ReturnValue :type "HitResult Structure"))
  (bind _returnvalue (`self.GetController`))
  (bind (_location _rotation) (`Controller.GetPlayerViewPoint` _returnvalue))
  (`/Engine/EditorBlueprintResources/StandardMacros.IsValid` _returnvalue
    (:`Is Valid`
      (bind _outhit (`KismetSystemLibrary.LineTraceSingle` _location (+ _location (* (`KismetMathLibrary.Conv_RotatorToVector` _rotation) (`self.TraceLength`))) "TraceTypeQuery1"))
      (return _outhit))))

(fn `SetDecalSize`
  (params (DecalSize :type "Float (double-precision)"))
  (set `self.DecalSize` (`KismetMathLibrary.FClamp` DecalSize 0.0 (`self.MaxDecalSize`)))
  (bind _isrtruntimedecalcomponent (`self.ISRTRuntimeDecalComponent`)
    (:`then`
      (`ISRTRuntimeDecalComponent.SetDecalSize` _isrtruntimedecalcomponent (`KismetMathLibrary.Conv_DoubleToVector` (`self.DecalSize`))))
    (:`else`)))

(fn `SetSelectedTexture`
  (params (SelectedTexture :type "Texture2D Object Reference"))
  (set `self.SelectedTexture` SelectedTexture)
  (bind _playerdecalmaterial (`self.PlayerDecalMaterial`)
    (:`then`
      (`MaterialInstanceDynamic.SetTextureParameterValue` _playerdecalmaterial "Texture" (`self.SelectedTexture`)))
    (:`else`)))

(fn `UserConstructionScript`)